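; Chat client actor that turns a chatbot's shopping spec into a product suggestion card on screen.
; On the chatbot's spec event, it parses semicolon-separated key=value text into suggest flag, category and budget range.
; When suggestion is on, it scans the catalog DataTable for the best-scoring row, though the budget score overwrites the category bonus.
; A match opens a suggestion card widget; a negative best score sends a no-match message back to the chatbot.
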(event `self.ReceiveBeginPlay`
  (add `ChatBotComponent.OnSpecJson` (`self.ChatBot`) (delegate `CustomEvent`)))

(event `CustomEvent`
  (params (JsonSpec :type String))
  (`KismetSystemLibrary.PrintString` JsonSpec true true (struct :`G` 0.66 :`B` 1.0 :`A` 1.0) 10.0)
  (for _array_element (`KismetStringLibrary.ParseIntoArray` JsonSpec ";")
    (bind (_lefts _rights) (`KismetStringLibrary.Split` _array_element "="))
    (switch `string` (`KismetStringLibrary.ToLower` _lefts)
      (:`suggest`
        (bind _output_get (set `self.Suggest` (== _rights "1")))
        (`KismetSystemLibrary.PrintString` (`KismetStringLibrary.Conv_BoolToString` _output_get) true true (struct :`G` 0.66 :`B` 1.0 :`A` 1.0) 10.0))
      (:`category`
        (bind _output_get_2 (set `self.Category` _rights))
        (`KismetSystemLibrary.PrintString` _output_get_2 true true (struct :`G` 0.66 :`B` 1.0 :`A` 1.0) 10.0))
      (:`budget_min`
        (bind _returnvalue (`KismetStringLibrary.Conv_StringToDouble` _rights))
        (set `self.BudgetMin` _returnvalue))
      (:`budget_max`
        (set `self.BudgetMax` _returnvalue))))
  (bind (_found _bestrow) (`self.Func_RecomendOne`))
  (if _found
    (bind _returnvalue_2 (`|CreateWidget` "/Game/UI/Widgets/WBP_SuggestionCard.WBP_SuggestionCard_C" null (`KismetTextLibrary.Conv_StringToText` (`.ItemName_23_0D099CAA46944E9F084F48988031743D` (break `/Game/Blueprints/Structs/Struct_CatalogItem` _bestrow)))))
    (`UserWidget.AddToViewport` _returnvalue_2 0)))

(fn `Func_RecomendOne`
  (returns (Found :type Boolean) (BestRow :type "/Game/Blueprints/Structs/Struct_CatalogItem Structure"))
  (locals (Score :type "Float (double-precision)") (BestScore :type "Float (double-precision)") (BestRowLocal :type "/Game/Blueprints/Structs/Struct_CatalogItem Structure") (Mid :type "Float (double-precision)"))
  (bind _dt_catalog (`self.DT_Catalog`))
  (if (`self.Suggest`)
    (set `local.Mid` (select `bool` (> (`self.BudgetMax`) 0.0) :`false` (`self.BudgetMin`) :`true` (/ (+ (`self.BudgetMin`) (`self.BudgetMax`)) 2.0)))
    (bind _outrownames (`DataTableFunctionLibrary.GetDataTableRowNames` _dt_catalog))
    (for _array_element _outrownames
      (bind _returnvalue (`|GetDataTableRow` _dt_catalog _array_element)
        (:`then`
          (bind _output_get (set `local.Score` 0.0))
          (bind (_id _itemname _category _styletags _dimensions _price) (break `/Game/Blueprints/Structs/Struct_CatalogItem` _returnvalue))
          (set `local.Score` (+ _output_get (select `bool` (== _category (`self.Category`)) :`true` 25.0)))
          (set `local.Score` (select `bool` (and (>= _price (`self.BudgetMin`)) (or (== (`self.BudgetMax`) 0.0) (<= _price (`self.BudgetMax`)))) :`false` (`KismetMathLibrary.FClamp` (/ (- _price (`local.Mid`)) 1000.0) 0.0 -15.0) :`true` 15.0))
          (if (> (`local.Score`) (`local.BestScore`))
            (set `local.BestScore` (`local.Score`))
            (set `local.BestRowLocal` _returnvalue)))))
    (if (>= (`local.BestScore`) 0.0)
      (return true (`local.BestRowLocal`))
      (else
        (`ChatBotComponent.SendUserMessage` (`self.ChatBot`) "[CATALOG_NO_MATCH]")
        (return false)))
    (else
      (return false))))

(fn `UserConstructionScript`)